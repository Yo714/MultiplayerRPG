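; WolfSpawn_BP is a spawner in Shinbi's PeaceOut ability content that summons a staggered arc of wolves around its HitDamage component.
; On BeginPlay it runs the parent logic, then calls SpawnWolf at evenly stepped angles with short delays between spawns.
; SpawnWolf uses sine and cosine to place each BP_Wolf at a raised radial offset, yawed toward the center, and always spawns regardless of collision.
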(event `self.ReceiveBeginPlay`
  (`parent.ReceiveBeginPlay`)
  (`self.SpawnWolf` 500.0 200.0 30.0)
  (`KismetSystemLibrary.Delay` 0.1)
  (`self.SpawnWolf` 500.0 200.0 60.0)
  (`KismetSystemLibrary.Delay` 0.1)
  (`self.SpawnWolf` 500.0 200.0 90.0)
  (`KismetSystemLibrary.Delay` 0.1)
  (`self.SpawnWolf` 500.0 200.0 120.0)
  (`KismetSystemLibrary.Delay` 0.1)
  (`self.SpawnWolf` 500.0 200.0 150.0)
  (`KismetSystemLibrary.Delay` 0.1))

(fn `SpawnWolf`
  (params (Distance :type "Float (double-precision)") (Height :type "Float (double-precision)") (Angle :type "Float (double-precision)"))
  (bind _hitdamage (`self.HitDamage`))
  (bind (_returnvalue_x _returnvalue_y _returnvalue_z) (`KismetMathLibrary.BreakVector` (`SceneComponent.K2_GetComponentLocation` _hitdamage)))
  (bind _returnvalue (`KismetMathLibrary.MakeVector` (+ _returnvalue_x (* Distance (`KismetMathLibrary.DegSin` Angle))) (+ _returnvalue_y (* Distance (`KismetMathLibrary.DegCos` Angle))) (+ _returnvalue_z Height)))
  (bind (_returnvalue_roll _returnvalue_pitch _returnvalue_yaw) (`KismetMathLibrary.BreakRotator` (`KismetMathLibrary.MakeRotFromX` (- (`SceneComponent.K2_GetComponentLocation` _hitdamage) _returnvalue))))
  (`|SpawnActorFromClass` "/Game/Characters/Shinbi/GAS/PeaceOut/BP_Wolf.BP_Wolf_C" (`KismetMathLibrary.MakeTransform` _returnvalue (`KismetMathLibrary.MakeRotator` 0.0 0.0 _returnvalue_yaw)) "AlwaysSpawn" "MultiplyWithRoot" null null))

(fn `UserConstructionScript`)